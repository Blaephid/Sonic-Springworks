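; Eye drone Blueprint that repeatedly plays a level sequence, set in its EyeFlash settings, once triggered.
; Triggeron runs only while inactive, then sets IsActive and creates a single sequence player that every loop reuses.
; Each pass waits the sequence length (end frame over frame-rate numerator) plus TimeBetween, then replays while IsActive holds.
; Nothing in this Blueprint's graphs clears IsActive.
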(event EventBeginPlay)

(event Collision|EventActorBeginOverlap
  (params (OtherActor :type Actor%20Object%20Reference)))

(event EventTick
  (params (DeltaSeconds :type Float%20%28single-precision%29)))

(event EventTriggeron
  (bind _eye_flash (Variables|Default|GetEye%20Flash))
  (if (not (Variables|Default|GetIsActive))
    (Variables|Default|SetIsActive true)
    (bind _outactor (Sequencer|Player|CreateLevelSequencePlayer (.sequencetoactivate _eye_flash)))
    (Sequencer|Player|Play (Variables|/Script/LevelSequence.LevelSequenceActor|GetSequencePlayer _outactor) :!class /Script/MovieScene.MovieSceneSequencePlayer :!label _label)
    (Utilities|FlowControl|Delay (/ (Math|Conversions|ToFloat(Integer) (.value (.frame (Class|MovieSceneSequencePlayer|GetEndTime (Variables|/Script/LevelSequence.LevelSequenceActor|GetSequencePlayer _outactor))))) (Math|Conversions|ToFloat(Integer) (.numerator (.framerate (Class|MovieSceneSequencePlayer|GetEndTime (Variables|/Script/LevelSequence.LevelSequenceActor|GetSequencePlayer _outactor)))))))
    (Utilities|FlowControl|Delay (.timebetween _eye_flash))
    (if (Variables|Default|GetIsActive)
      (goto _label))))

(fn ConstructionScript)