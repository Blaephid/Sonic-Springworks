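; Level-design ladder that procedurally builds itself to a configurable Height, with placeholder teleport logic between its bottom and top triggers.
; The construction script positions the top trigger, then loops to add paired side meshes, stretched to fit fractional heights, and evenly spaced rungs.
; Trigger overlap events currently do nothing; the code that would set teleport flags and move the overlapping actor is disconnected and has empty casts.
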(event OnComponentBeginOverlap(BottomTrigger)
  (params (OverlappedComponent :type Primitive%20Component%20Object%20Reference) (OtherActor :type Actor%20Object%20Reference) (OtherComp :type Primitive%20Component%20Object%20Reference) (OtherBodyIndex :type Integer) (bFromSweep :type Boolean) (SweepResult :type Hit%20Result%20Structure%20%28by%20ref%29))
  (if (Variables|Default|GetCanTeleportUp)
    _))

(event OnComponentBeginOverlap(TopTrigger1)
  (params (OverlappedComponent :type Primitive%20Component%20Object%20Reference) (OtherActor :type Actor%20Object%20Reference) (OtherComp :type Primitive%20Component%20Object%20Reference) (OtherBodyIndex :type Integer) (bFromSweep :type Boolean) (SweepResult :type Hit%20Result%20Structure%20%28by%20ref%29))
  (if (Variables|Default|GetCanTeleportDown)
    _))

(event OnComponentEndOverlap(BottomTrigger)
  (params (OverlappedComponent :type Primitive%20Component%20Object%20Reference) (OtherActor :type Actor%20Object%20Reference) (OtherComp :type Primitive%20Component%20Object%20Reference) (OtherBodyIndex :type Integer)))

(event OnComponentEndOverlap(TopTrigger1)
  (params (OverlappedComponent :type Primitive%20Component%20Object%20Reference) (OtherActor :type Actor%20Object%20Reference) (OtherComp :type Primitive%20Component%20Object%20Reference) (OtherBodyIndex :type Integer)))

(fn ConstructionScript
  (bind _top_trigger1 (Variables|Default|GetTop%20Trigger1))
  (bind _bottom_trigger (Variables|Default|GetBottom%20Trigger))
  (bind _returnvalue (Transformation|GetWorldLocation _top_trigger1))
  (Utilities|FlowControl|Sequence
    (:then_0
      ;[0 0 0] Setting trigger at top of ladder.
      (bind _output_get (Variables|Default|SetHeight (Math|Float|Clamp(Float) (Variables|Default|GetHeight) 1.0 (Variables|Default|GetHeight))))
      (Transformation|SetWorldLocation (Variables|Default|GetTop%20Trigger1) (Math|Vector|MakeVector (.x _returnvalue) (.y _returnvalue) (.z (+ (Transformation|GetWorldLocation _bottom_trigger) (* (+ (* _output_get (Variables|Default|GetHeightModifierFromMesh)) -2e+01) (Math|Vector|GetUpVector _bottom_trigger))))) false false))
    (:then_2
      ;[0 0 0] Adding ladder sides, from bottom to set height
      ;;[0 0 0] Add a new mesh to side for every whole number of height.
      (bind _output_get_2 (LocalVariables|SetScaleModi (/ (Variables|Default|GetHeight) (Math|Float|Truncate (Variables|Default|GetHeight)))))
      (bind _output_get_3 (LocalVariables|SetScaleTracking 0.0))
      (while (<= _output_get_3 (- (Variables|Default|GetHeight) _output_get_2))
        ;;[0 0 0] Add Mesh On Either Side
        (CallFunction|AddLadderSideatVector (Math|Vector|MakeVector 0.0 0.0 (+ (Variables|Default|GetStartSidesOffset) (* (LocalVariables|GetScaleTracking) (Variables|Default|GetHeightModifierFromMesh)))) "0.000000,-90.000000,0.000000" (Math|Vector|MakeVector 1.0 1.0 (LocalVariables|GetScaleModi)))
        (CallFunction|AddLadderSideatVector (Math|Vector|MakeVector 0.0 0.0 (+ (Variables|Default|GetStartSidesOffset) (* (LocalVariables|GetScaleTracking) (Variables|Default|GetHeightModifierFromMesh)))) "0.000000,90.000000,0.000000" (Math|Vector|MakeVector 1.0 1.0 (LocalVariables|GetScaleModi)))
        (LocalVariables|SetScaleTracking (+ (LocalVariables|GetScaleModi) (LocalVariables|GetScaleTracking)))))
    (:then_3
      ;[0 0 0] Adding Rungs up ladder (4 per needed sides)
      (bind _output_get_4 (LocalVariables|SetRungModi (* (/ 1.0 5.0) (LocalVariables|GetScaleModi))))
      (bind _output_get_5 (LocalVariables|SetRungTracking _output_get_4))
      (while (<= _output_get_5 (- (Variables|Default|GetHeight) _output_get_4))
        (CallFunction|AddLadderRungatVector (Math|Vector|MakeVector 0.0 0.0 (* (LocalVariables|GetRungTracking) (Variables|Default|GetHeightModifierFromMesh))) "90.000000,0.000000,0.000000" "0.050000,0.050000,0.500000")
        (LocalVariables|SetRungTracking (+ (LocalVariables|GetRungTracking) (LocalVariables|GetRungModi)))))))

(fn AddLadderSideatVector
  (params (Vector :type Vector) (Rotation :type Rotator) (Scale :type Vector))
  (bind _returnvalue (AddComponent|AddStaticMeshComponent false (Math|Transform|MakeTransform Vector Rotation Scale)))
  (Components|StaticMesh|SetStaticMesh _returnvalue (Variables|Default|GetLadderSides)))

(fn AddLadderRungatVector
  (params (Vector :type Vector) (Rotation :type Rotator) (Scale :type Vector))
  (bind _returnvalue (AddComponent|AddStaticMeshComponent false (Math|Transform|MakeTransform Vector Rotation Scale)))
  (Components|StaticMesh|SetStaticMesh _returnvalue (Variables|Default|GetLadder%20Rungs)))