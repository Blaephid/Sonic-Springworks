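; Level-design prop that carries a configurable mesh, name, information, image and particle look, with a WBP_PopUp widget to present the data.
; The construction script applies mesh and particle settings and fills the widget, which BeginPlay refills and hides.
; Tick yaws the widget toward Player while Active.
; Trigger overlap events are empty; the animated show/hide logic is disconnected and its casts lack a class, so the popup stays hidden.
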(event OnComponentBeginOverlap(TriggerEnter)
  (params (OverlappedComponent :type Primitive%20Component%20Object%20Reference) (OtherActor :type Actor%20Object%20Reference) (OtherComp :type Primitive%20Component%20Object%20Reference) (OtherBodyIndex :type Integer) (bFromSweep :type Boolean) (SweepResult :type Hit%20Result%20Structure%20%28by%20ref%29)))

(event OnComponentEndOverlap(TriggerEnter)
  (params (OverlappedComponent :type Primitive%20Component%20Object%20Reference) (OtherActor :type Actor%20Object%20Reference) (OtherComp :type Primitive%20Component%20Object%20Reference) (OtherBodyIndex :type Integer)))

(event EventBeginPlay
  (Rendering|SetVisibility (Variables|Default|GetWidget) false false)
  (CallFunction|UpdateWidgetText))

(event Collision|EventActorBeginOverlap
  (params (OtherActor :type Actor%20Object%20Reference)))

(event EventTick
  (params (DeltaSeconds :type Float%20%28single-precision%29))
  (bind _returnvalue (Transformation|GetActorLocation))
  (bind _player (Variables|Default|GetPlayer))
  (bind _returnvalue_2 (Transformation|GetActorLocation _player))
  (bind _returnvalue_3 (Math|Vector|GetUnitDirection(Vector) _returnvalue _returnvalue_2))
  (bind (_x _y) (Math|Vector|BreakVector _returnvalue_3))
  (if (Variables|Default|GetActive)
    (Transformation|SetWorldRotation (Variables|Default|GetWidget) (Math|Rotator|MakeRotfromX (Math|Vector|MakeVector _x _y 0.0)) false false)))

(fn ConstructionScript
  (bind _particle (Variables|Default|GetParticle))
  (Utilities|FlowControl|Sequence
    (:then_0
      (Components|StaticMesh|SetStaticMesh (Variables|Default|GetStaticMesh) (Variables|Default|GetMesh)))
    (:then_1
      (CallFunction|UpdateWidgetText))
    (:then_2
      (Niagara|SetNiagaraVariable(LinearColor) _particle "Color" (Variables|Default|GetParticle%20Colour))
      (Niagara|SetNiagaraVariable(Float) _particle "Size" (Variables|Default|GetParticle%20Size)))))

(fn UpdateWidgetText
  (bind _aswbp_pop_up (Utilities|Casting|CastToWBP_PopUp (UserInterface|GetWidget (Variables|Default|GetWidget))))
  (Default|SetNameFunction _aswbp_pop_up (Variables|Default|GetName))
  (Default|SetInfoFunction _aswbp_pop_up (Variables|Default|GetInformation))
  (Default|SetImageFunction _aswbp_pop_up (Variables|Default|GetImage)))