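; Level design ruler actor that shows cover heights and distance measurements, rebuilt in the construction script as it is scaled.
; X and Y scale snap to half steps; the cover-height mesh stays fixed vertically, while an extension mesh 200 units up absorbs extra Z scale.
; PlaceLineOfMeasurementPairs walks each horizontal axis, using PlaceSpacingMeasurement to add paired 1-meter marker meshes on opposite edges at every second increment and near the ends.
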(event EventBeginPlay)

(event Collision|EventActorBeginOverlap
  (params (OtherActor :type Actor%20Object%20Reference)))

(event EventTick
  (params (DeltaSeconds :type Float%20%28single-precision%29)))

(fn ConstructionScript
  (bind _defaultsceneroot (Variables|Default|GetDefaultSceneRoot))
  (bind _obd_extendcover (Variables|Default|GetObD_ExtendCover))
  (bind _defaultsceneroot_2 (Variables|Default|GetDefaultSceneRoot))
  (bind _defaultsceneroot_3 (Variables|Default|GetDefaultSceneRoot))
  (bind _returnvalue (Transformation|GetWorldLocation _defaultsceneroot_2))
  (bind _returnvalue_2 (Transformation|GetWorldScale _defaultsceneroot_3))
  (Utilities|FlowControl|Sequence
    (:then_0
      ;[0 0 0 1 32] Set Middle Cover Ruler to increments of 0.5, and lock vertical
      (LocalVariables|SetYScaleIncrement (/ (Math|Conversions|ToFloat(Integer) (Math|Float|Round (* (.y _returnvalue_2) 2.0))) 2.0))
      (LocalVariables|SetXScaleIncrement (/ (Math|Conversions|ToFloat(Integer) (Math|Float|Round (* (.x _returnvalue_2) 2.0))) 2.0))
      (Transformation|SetWorldScale3D (Variables|Default|GetObD_CoverHeights) (Math|Vector|MakeVector (LocalVariables|GetXScaleIncrement) (LocalVariables|GetYScaleIncrement) 1.0))
      ;[0 0 0 1 32] Extend only white grid up on z scale.
      (Transformation|SetWorldScale3D _obd_extendcover (Math|Vector|MakeVector (LocalVariables|GetXScaleIncrement) (LocalVariables|GetYScaleIncrement) (Math|Float|Max(Float) (- (.z (Transformation|GetWorldScale (Variables|Default|GetDefaultSceneRoot))) 1.0) 0.0)))
      (Variables|Default|SetActorLocation _returnvalue)
      (Transformation|SetWorldLocation _obd_extendcover (+ (* (Math|Vector|GetUpVector _defaultsceneroot_2) 2e+02) _returnvalue) false false))
    (:then_1
      ;[0 0 0 1 24] Setting Values for Measurement Lines
      (LocalVariables|SetActorForward (Math|Vector|GetForwardVector _defaultsceneroot))
      (LocalVariables|SetActorRight (Math|Vector|GetRightVector _defaultsceneroot))
      (LocalVariables|SetXScaleIncrementHalfPoint (/ (LocalVariables|GetXScaleIncrement) 2.0))
      (LocalVariables|SetYScaleIncrementHalfPoint_0 (/ (LocalVariables|GetYScaleIncrement) 2.0))
      ;[0 0 0 1 32] Place distance measurements along extents. X and Y Dimensions.
      (Utilities|FlowControl|Sequence
        (:then_0
          (CallFunction|PlaceLineOfMeasurementPairs (LocalVariables|GetActorForward) (LocalVariables|GetXScaleIncrement) (LocalVariables|GetXScaleIncrementHalfPoint) (LocalVariables|GetYScaleIncrement) (LocalVariables|GetYScaleIncrementHalfPoint_0) (LocalVariables|GetActorRight) 1 1))
        (:then_1
          (CallFunction|PlaceLineOfMeasurementPairs (LocalVariables|GetActorRight) (LocalVariables|GetYScaleIncrement) (LocalVariables|GetYScaleIncrementHalfPoint_0) (LocalVariables|GetXScaleIncrement) (LocalVariables|GetXScaleIncrementHalfPoint) (LocalVariables|GetActorForward) 2 2))))))

(fn PlaceSpacingMeasurement
  (params (Actor%20Direction :type Vector) (Halfpoint :type Float%20%28double-precision%29) (Index :type Integer) (MeshToSet :type Static%20Mesh%20Object%20Reference) (Offset :type Vector))
  (bind _returnvalue (AddComponent|AddStaticMeshComponent false))
  (bind _output_get (LocalVariables|SetCurrentMeshSetting _returnvalue))
  (Transformation|SetWorldScale3D _output_get "1.000000,1.000000,1.000000")
  (Transformation|SetWorldLocation (LocalVariables|GetCurrentMeshSetting) (+ Offset (+ (Variables|Default|GetActorLocation) (* (* (- (/ (Math|Conversions|ToFloat(Integer) Index) 2.0) Halfpoint) Actor%20Direction) 1e+02))) false false)
  ;[0 0 0] Set Mesh
  (Components|StaticMesh|SetStaticMesh (LocalVariables|GetCurrentMeshSetting) MeshToSet))

(fn PlaceLineOfMeasurementPairs
  (params (DirectionOfLine :type Vector) (AxisScale :type Float%20%28double-precision%29) (Halfpoint :type Float%20%28double-precision%29) (OtherAxisScale :type Float%20%28double-precision%29) (OtherAxisHalfPoint :type Float%20%28double-precision%29) (PerpendicularOfLine :type Vector) (First%20Index :type Integer) (LastIndexOffset :type Integer))
  (bind _returnvalue (* AxisScale 2.0))
  (bind _returnvalue_2 (Utilities|Operators|Subtract OtherAxisScale OtherAxisHalfPoint 0.5))
  (bind _1metermesh (Variables|Default|Get1MeterMesh))
  (bind _returnvalue_3 (Math|Float|Truncate _returnvalue))
  (bind _returnvalue_4 (* PerpendicularOfLine _returnvalue_2 1e+02))
  (bind _returnvalue_5 (- _returnvalue_3 LastIndexOffset))
  ;[0 0 0] Loop along length
  (for _index (range First%20Index _returnvalue_5)
    (LocalVariables|SetCurrentIndex _index)
    ;[0 0 0] Only place if a second increment, or the first or last point.
    (if (or (== (.Remainder (Math|Float|Division(WholeandRemainder) (Math|Conversions|ToFloat(Integer) (LocalVariables|GetCurrentIndex)) 2.0)) 0.0) (or (== _returnvalue_5 (LocalVariables|GetCurrentIndex)) (== 1 (LocalVariables|GetCurrentIndex))))
      ;[0 0 0 1 24] Place a measurement on the left and right sides according to the other scale.
      (Utilities|FlowControl|Sequence
        (:then_0
          (CallFunction|PlaceSpacingMeasurement DirectionOfLine Halfpoint (LocalVariables|GetCurrentIndex) _1metermesh _returnvalue_4))
        (:then_1
          (CallFunction|PlaceSpacingMeasurement DirectionOfLine Halfpoint (LocalVariables|GetCurrentIndex) _1metermesh (* _returnvalue_4 -1.0)))))))