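; Breakable actor trigger that a SpringPawn smashes by overlapping its box during one of the VulnerableAttacks states.
; A one-shot gate then checks the pawn's animation state and, if it matches, overrides its velocity with the PlayerLaunch result.
; The base mesh, optionally physics-simulated from BeginPlay, is hidden with physics and collision disabled, and a BrkActor child actor is spawned at the actor's transform.
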(event OnComponentBeginOverlap(Box)
  (params (OverlappedComponent :type Primitive%20Component%20Object%20Reference) (OtherActor :type Actor%20Object%20Reference) (OtherComp :type Primitive%20Component%20Object%20Reference) (OtherBodyIndex :type Integer) (bFromSweep :type Boolean) (SweepResult :type Hit%20Result%20Structure%20%28by%20ref%29))
  (bind _returnvalue (Transformation|GetActorTransform))
  (bind _base_mesh (Variables|Default|GetBase_Mesh))
  (bind _asspring_pawn (Utilities|Casting|CastToSpringPawn OtherActor))
  (if (Utilities|Map|Contains (Variables|Default|GetVulnerable%20Attacks) (Variables|/Game/SonicSpringworks/System/SpringPawn.SpringPawn_C|GetAtk_State _asspring_pawn))
    (Utilities|FlowControl|DoOnce false
      (:Completed
        (if (Default|CheckAnimState _asspring_pawn "NewEnumerator2")
          (Default|SetVelocity _asspring_pawn (|PlayerLaunch _asspring_pawn) true true false false)
          (Physics|SetSimulatePhysics _base_mesh false)
          (Collision|SetCollisionEnabled _base_mesh "NoCollision")
          (Rendering|SetVisibility _base_mesh false false)
          (bind _returnvalue_2 (AddComponent|AddChildActorComponent false _returnvalue))
          (Transformation|SetWorldTransform _returnvalue_2 _returnvalue false false)
          (ChildActorComponent|SetChildActorClass _returnvalue_2 (Variables|Default|GetBrk%20Actor)))))))

(event EventBeginPlay
  (Physics|SetSimulatePhysics (Variables|Default|GetBase_Mesh) (Variables|Default|GetPhysics?)))

(fn ConstructionScript)