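; EggSpring is a spring object that launches an overlapping SpringPawn along its up vector and applies its damage type.
; On touch, it cancels the pawn's action, snaps it to the spring mesh, launches it by LaunchStrength, briefly locks input and sets its jump count.
; It also plays the spring animation and sound and sets the pawn's animation state.
; The construction script displays the strength and draws the predicted launch path as a persistent debug preview.
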(event OnComponentBeginOverlap(Box)
  (params (OverlappedComponent :type Primitive%20Component%20Object%20Reference) (OtherActor :type Actor%20Object%20Reference) (OtherComp :type Primitive%20Component%20Object%20Reference) (OtherBodyIndex :type Integer) (bFromSweep :type Boolean) (SweepResult :type Hit%20Result%20Structure%20%28by%20ref%29))
  (bind _asspring_pawn (Utilities|Casting|CastToSpringPawn OtherActor))
  (Variables|Default|SetPawn _asspring_pawn)
  (CallFunction|SpringTouched)
  (Default|DmgFunc _asspring_pawn (Variables|Default|GetDmgType)))

(event Custom|SpringTouched
  (Utilities|FlowControl|Sequence
    (:then_0
      (|TouchLogic))
    (:then_1
      (|TouchFX))))

(fn ConstructionScript
  (Transformation|SetRelativeLocation (Variables|Default|GetSkeletalMesh) (Math|Vector|MakeVector 0.0 0.0 (Variables|Spring|GetRelativeOffsetZ)) false false)
  (Rendering|Components|TextRender|SetText (Variables|Default|GetTextRender) (Utilities|Text|ToText(Float) (Variables|Spring|GetLaunchStrength) "HalfToEven" false true 1 324 1 2))
  (Rendering|Debug|FlushPersistentDebugLines)
  (Class|GameplayStatics|BlueprintPredictProjectilePathAdvanced (Utilities|Struct|MakePredictProjectilePathParams (Transformation|GetWorldLocation (Variables|Default|GetSkeletalMesh)) (* (Transformation|GetActorUpVector) (Variables|Spring|GetLaunchStrength) 1e+03) false 0.0 1.0 true "ECC_WorldStatic" "ObjectTypeQuery1" 0 2e+01 0.0 "Persistent" 1.0 true)))